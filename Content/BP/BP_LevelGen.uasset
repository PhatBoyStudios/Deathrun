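; BP_LevelGen is a level generator that lays out three level piece Blueprints in a random order, each spawned once.
; Every Tick, PickPiece rolls a random piece ID and SpawnPiece spawns it unless its Done flag is set.
; Each spawn advances Position 1000 units along Y.
; The all-done check on Tick does nothing and FullDone is never set here, so rolling continues after completion.
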(event `self.ReceiveTick`
  (params (DeltaSeconds :type "Float (single-precision)"))
  (`self.PickPiece`)
  (if (and (and (`self.1Done`) (`self.2Done`)) (`self.3Done`))
    _))

(fn `PickPiece`
  (if (not (`self.FullDone`))
    (switch `int` (`KismetMathLibrary.RandomIntegerInRange` 1 3)
      (:`1`
        (`self.SpawnPiece` 1))
      (:`2`
        (`self.SpawnPiece` 2))
      (:`3`
        (`self.SpawnPiece` 3)))))

(fn `SpawnPiece`
  (params (ID :type Integer))
  (if (== ID 1)
    (if (`self.1Done`)
      (return)
      (else
        (`|SpawnActorFromClass` "/Game/BP/BP_LevelPiece1.BP_LevelPiece1_C" (`KismetMathLibrary.MakeTransform` (`self.Position`)) "Undefined" "OverrideRootScale" null null)
        (set `self.1Done` true)
        (set `self.Position` (+ (`self.Position`) (0.0 1000.0 0.0)))))
    (elif (== ID 2)
      (if (`self.2Done`)
        (return)
        (else
          (`|SpawnActorFromClass` "/Game/BP/BP_LevelPiece2.BP_LevelPiece2_C" (`KismetMathLibrary.MakeTransform` (`self.Position`)) "Undefined" "OverrideRootScale" null null)
          (set `self.2Done` true)
          (set `self.Position` (+ (`self.Position`) (0.0 1000.0 0.0)))))
      (elif (== ID 3)
        (if (`self.3Done`)
          (return)
          (else
            (`|SpawnActorFromClass` "/Game/BP/BP_LevelPiece3.BP_LevelPiece3_C" (`KismetMathLibrary.MakeTransform` (`self.Position`)) "Undefined" "OverrideRootScale" null null)
            (set `self.3Done` true)
            (set `self.Position` (+ (`self.Position`) (0.0 1000.0 0.0)))))
        (else
          (return))))))

(fn `UserConstructionScript`)